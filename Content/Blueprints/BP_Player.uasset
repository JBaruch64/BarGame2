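; Player Blueprint for what appears to be a bartending game, handling the codex and switching between bar and fridge views.
; Enhanced Input toggles the codex widget and blends between tagged CameraActors, swapping fridge and bottle-bar UI.
; Returning to the bar copies FridgeItems into a new selected-ingredients widget.
; BeginPlay and look-up/mouse-look events are empty; their logic, including input, HUD and starting-camera setup, is disconnected.
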(event `EnhancedInput|/Game/Input/IA_ToggleCodex`
  (params (ActionValue :type Boolean) (ElapsedSeconds :type "Float (double-precision)") (TriggeredSeconds :type "Float (double-precision)") (InputAction :type "InputAction Object Reference" :default "/Game/Input/IA_ToggleCodex.IA_ToggleCodex"))
  ;[0.1106 0.08182 0.15 0.5] Codex Toggle
  (:`Started`
    (if (`self.IsCodexOpen`)
      (`Widget.RemoveFromParent` (`self.CodexWidget`))
      (set `self.IsCodexOpen` false)
      (set `PlayerController.bShowMouseCursor` true (`GameplayStatics.GetPlayerController` 0))
      (else
        (bind _returnvalue (`|CreateWidget` "/Game/UI/WBP_Codex.WBP_Codex_C" (`GameplayStatics.GetPlayerController` 0)))
        (bind _output_get (set `self.CodexWidget` _returnvalue))
        (`UserWidget.AddToViewport` _output_get 0)
        (set `self.IsCodexOpen` true)
        (set `PlayerController.bShowMouseCursor` true (`GameplayStatics.GetPlayerController` 0))))))

(event `self.ReceiveBeginPlay`)

(event `EnhancedInput|/Game/Input/IA_MouseLook`
  (params (ActionValue :type "Float (double-precision)") (ElapsedSeconds :type "Float (double-precision)") (TriggeredSeconds :type "Float (double-precision)") (InputAction :type "InputAction Object Reference" :default "/Game/Input/IA_MouseLook.IA_MouseLook"))
  ;[0 0.15 0.136 0.5] Mouse Look Around
)

(event `EnhancedInput|/Game/Input/IA_LookUp`
  (params (ActionValue :type "Float (double-precision)") (ElapsedSeconds :type "Float (double-precision)") (TriggeredSeconds :type "Float (double-precision)") (InputAction :type "InputAction Object Reference" :default "/Game/Input/IA_LookUp.IA_LookUp"))
  ;[0.03518 0.15 0 0.5] LookUp (W)
)

(event `EnhancedInput|/Game/Input/IA_LookDown`
  (params (ActionValue :type "Float (double-precision)") (ElapsedSeconds :type "Float (double-precision)") (TriggeredSeconds :type "Float (double-precision)") (InputAction :type "InputAction Object Reference" :default "/Game/Input/IA_LookDown.IA_LookDown"))
  ;[0.1486 0.15 0.000259 0.5] (S) (turn around)
  (:`Started`
    (if (`self.bFridgeOpen`)
      (bind _outactors (`GameplayStatics.GetAllActorsOfClassWithTag` "/Script/Engine.CameraActor" "BarCamera"))
      (`PlayerController.SetViewTargetWithBlend` (`GameplayStatics.GetPlayerController` 0) (`|GetArrayItem` _outactors) 0.5 "VTBlend_Linear" 0.0 false)
      (set `self.bFridgeOpen` false)
      (`Widget.RemoveFromParent` (`self.FridgeWidgetRef`))
      (bind _returnvalue (`|CreateWidget` "/Game/Blueprints/UIClick/WBP_SelectedIngredients.WBP_SelectedIngredients_C" (`GameplayStatics.GetPlayerController` 0)))
      (bind _output_get (set `self.SelectedIngredientsRef` _returnvalue))
      (`UserWidget.AddToViewport` _output_get 0)
      (for _array_element (`self.FridgeItems`)
        (`/Game/Blueprints/UIClick/WBP_SelectedIngredients.AddIngredient` (`self.SelectedIngredientsRef`) _array_element))
      (`Widget.SetVisibility` (`self.BottleBarWidgetRef`) "Visible")
      (else
        (bind _outactors_2 (`GameplayStatics.GetAllActorsOfClassWithTag` "/Script/Engine.CameraActor" "FridgeCamera"))
        (`PlayerController.SetViewTargetWithBlend` (`GameplayStatics.GetPlayerController` 0) (`|GetArrayItem` _outactors_2) 0.5 "VTBlend_Linear" 0.0 false)
        (set `self.bFridgeOpen` true)
        (bind _returnvalue_2 (`|CreateWidget` "/Game/Blueprints/UIClick/WBP_Fridge.WBP_Fridge_C" (`GameplayStatics.GetPlayerController` 0)))
        (bind _output_get_2 (set `self.FridgeWidgetRef` _returnvalue_2))
        (`UserWidget.AddToViewport` _output_get_2 0)
        (`Widget.SetVisibility` (`self.BottleBarWidgetRef`) "Hidden")))))

(fn `SetupInput`
  (`EnhancedInputSubsystemInterface.AddMappingContext` (pcsubsystem `EnhancedInputLocalPlayerSubsystem` (`GameplayStatics.GetPlayerController` 0)) "/Game/Input/IMC_Controls.IMC_Controls" 0 (struct)))

(fn `UserConstructionScript`)